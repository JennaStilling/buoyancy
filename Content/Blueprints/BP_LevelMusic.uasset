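; BP_LevelMusic is an actor that plays a level's music track and fades it out on request.
; BeginPlay calls StartMusic, which spawns LevelMusic as a 2D sound, stores it in MusicRef and plays it from the start.
; The MusicTransition event, not called within this Blueprint, fades that sound out over FadeValue and schedules a stop after the same delay.
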(event Custom|MusicTransition
  (bind _musicref (Variables|Default|GetMusicRef))
  (bind _fadevalue (Variables|Default|GetFadeValue))
  (Audio|Components|Audio|FadeOut _musicref _fadevalue 0.0 "Linear" :!class /Script/Engine.AudioComponent)
  (Audio|Components|Audio|StopDelayed _musicref _fadevalue))

(event Custom|StartMusic
  (bind _returnvalue (Audio|SpawnSound2D (Variables|Default|GetLevelMusic) 1.0 1.0 0.0 0))
  (bind _output_get (Variables|Default|SetMusicRef _returnvalue))
  (Audio|Components|Audio|Play _output_get 0.0))

(event EventBeginPlay
  (CallFunction|StartMusic))

(event Collision|EventActorBeginOverlap
  (params (OtherActor :type Actor%20Object%20Reference)))

(event EventTick
  (params (DeltaSeconds :type Float%20%28single-precision%29)))

(fn ConstructionScript)