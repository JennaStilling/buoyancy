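; BPP_EnemyParent is a parent Blueprint for enemies that tracks health, reacts to damage and handles death.
; The Damage event subtracts from Health, then either calls DamageEffect or, at zero or below, tells its BP_gateway to decrement its remaining count and calls Die.
; Die routes to DeathEffect, which destroys the actor, while DamageEffect is an empty hook.
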(event Custom|Damage
  (params (Damage :type Integer))
  (bind _output_get (Variables|Default|SetHealth (- (Variables|Default|GetHealth) Damage)))
  (if (<= _output_get 0)
    (bind _asbp_gateway (Utilities|Casting|CastToBP_gateway (Variables|Default|GetGateway))
      (:then
        (Default|DecrementLeft _asbp_gateway))
      (:CastFailed
        _))
    (CallFunction|Die)
    (else
      (CallFunction|DamageEffect))))

(event Custom|Die
  (CallFunction|DeathEffect))

(event Custom|DamageEffect)

(event Custom|DeathEffect
  (Actor|DestroyActor))

(event EventBeginPlay)

(event Collision|EventActorBeginOverlap
  (params (OtherActor :type Actor%20Object%20Reference)))

(event EventTick
  (params (DeltaSeconds :type Float%20%28single-precision%29)))

(fn ConstructionScript)