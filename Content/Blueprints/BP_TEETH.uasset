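; BP_TEETH is an AI enemy pawn that wanders, chases the player on sight and destroys the player character on capsule contact.
; While not aggroed, Tick issues delayed moves to random reachable points, playing a looping teeth animation.
; Pawn sensing sets Aggro and starts an AI move toward the player, clearing Aggro if that fails.
; Damage and death effects print debug text before calling parent logic.
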(event OnSeePawn(PawnSensing)
  (params (Pawn :type Pawn%20Object%20Reference))
  (Utilities|Casting|CastToBP_ThirdPersonCharacter Pawn)
  (Variables|Default|SetAggro true)
  (CallFunction|ChasePlayer)
  (Components|Animation|PlayAnimation (Variables|Character|GetMesh) "/Game/Animations/Teeth/ANIM_teeth.ANIM_teeth" true))

(event OnComponentHit(CapsuleComponent)
  (params (HitComponent :type Primitive%20Component%20Object%20Reference) (OtherActor :type Actor%20Object%20Reference) (OtherComp :type Primitive%20Component%20Object%20Reference) (NormalImpulse :type Vector :default "0, 0, 0") (Hit :type Hit%20Result%20Structure%20%28by%20ref%29))
  (bind _asbp_third_person_character (Utilities|Casting|CastToBP_ThirdPersonCharacter OtherActor))
  (Actor|DestroyActor _asbp_third_person_character))

(event Custom|ChasePlayer
  (if (Variables|Default|GetAggro)
    (AI|AIMoveTo self "0, 0, 0" (Game|Player|GetPlayerPawn 0) (Variables|Default|GetStopDistance) false
      (:OnFail
        (Variables|Default|SetAggro false)))))

(event EventBeginPlay
  (|CallParentFunction) ; This node is disabled and will not be called.\nDrag off pins to build functionality.
)

(event Collision|EventActorBeginOverlap
  (params (OtherActor :type Actor%20Object%20Reference))
  (|CallParentFunction OtherActor) ; This node is disabled and will not be called.\nDrag off pins to build functionality.
)

(event EventTick
  (params (DeltaSeconds :type Float%20%28single-precision%29))
  (|CallParentFunction DeltaSeconds)
  (if (not (Variables|Default|GetAggro))
    (Utilities|FlowControl|Delay 2.0)
    (AI|AIMoveTo self (.RandomLocation (AI|Navigation|GetRandomReachablePointinRadius (Transformation|GetActorLocation) 1e+03 0 0)) 0 5.0 false
      (:then
        (Components|Animation|PlayAnimation (Variables|Character|GetMesh) "/Game/Animations/Teeth/ANIM_teeth.ANIM_teeth" true))
      (:OnSuccess
        (Audio|Components|Audio|Stop (Variables|Character|GetMesh))))))

(event EventDamageEffect
  (Development|PrintString (Utilities|String|Append "TEETH Health:" (Utilities|String|ToString(Integer) (Variables|Default|GetHealth))))
  (|CallParentFunction))

(event EventDeathEffect
  (Development|PrintString "dedest")
  (|CallParentFunction))

(fn ConstructionScript
  (|CallParentFunction))