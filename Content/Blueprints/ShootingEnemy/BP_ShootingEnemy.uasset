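; BP_ShootingEnemy is an enemy that turns toward the player and lobs projectiles when within ShootingRange.
; Tick checks distance, yaws the enemy to face the player, and fires once the cooldown timer elapses.
; Each shot spawns a BP_ShootingEnemyProjectile, adds a projectile movement component, and sets a velocity predicted to hit the moving player after TimeToTarget.
; Damage and death events print debug text, then call the parent effects.
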(event Custom|Shoot
  (Variables|Default|SetTimePassed 0.0)
  (bind _returnvalue (Game|SpawnActorfromClass "/Game/blueprints/ShootingEnemy/BP_ShootingEnemyProjectile.BP_ShootingEnemyProjectile_C" (Transformation|GetActorTransform) "Undefined" "MultiplyWithRoot" 0 0))
  ;[1 1 1] Throws the Throwable at the player, with a specified air time (Time To Target)
  (bind _outlaunchvelocity (Class|GameplayStatics|SuggestProjectileVelocityMovingTarget (.location (Transformation|GetActorTransform)) (Game|GetPlayerCharacter 0) "0, 0, 0" 0.0 (Variables|Default|GetTimeToTarget) "None"))
  (bind _returnvalue_2 (AddComponent|AddProjectileMovementComponent _returnvalue))
  (Variables|/Script/Engine.MovementComponent|SetVelocity _returnvalue_2 _outlaunchvelocity))

(event EventDamageEffect
  (Development|PrintString (Utilities|String|Append "Enemy hit, Health: " (Utilities|String|ToString(Integer) (Variables|Default|GetHealth))))
  (|CallParentFunction))

(event EventTick
  (params (DeltaSeconds :type Float%20%28single-precision%29))
  (Variables|Default|SetTimePassed (+ (Variables|Default|GetTimePassed) DeltaSeconds))
  (if (Utilities|IsValid (Game|Player|GetPlayerPawn 0))
    (if (<= (Math|Vector|Distance(Vector) (Transformation|GetActorLocation (Game|Player|GetPlayerPawn 0)) (Transformation|GetActorLocation)) (Variables|Default|GetShootingRange))
      (CallFunction|FacePlayer)
      (if (<= (Variables|Default|GetShootingCoolDown) (Variables|Default|GetTimePassed))
        (CallFunction|Shoot)))))

(event EventDeathEffect
  (Development|PrintString "Ded")
  (|CallParentFunction))

(fn ConstructionScript)

(fn FacePlayer
  (Transformation|SetActorRotation (Math|Conversions|RotationFromXVector (Math|Vector|RotateVector (Math|Vector|Normalize (* (- (Transformation|GetActorLocation (Game|Player|GetPlayerPawn 0)) (Transformation|GetActorLocation)) "1.000000,1.000000,0.000000")) "0, 0, 0"))))