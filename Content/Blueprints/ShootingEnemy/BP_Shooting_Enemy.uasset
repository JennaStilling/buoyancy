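; BP_Shooting_Enemy is an enemy actor that turns toward the player within shooting range and has health.
; Tick tracks elapsed time, prints debug text and calls FacePlayer for horizontal-only rotation.
; Damage reduces health, calling empty effect hooks and destroying the actor at zero.
; Shoot spawns a projectile with a timed moving-target arc at the player, but its cooldown check is disconnected, so nothing here fires it.
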(event Custom|Die
  (CallFunction|DeathEffect)
  (Actor|DestroyActor))

(event Custom|Shoot
  (Variables|Default|SetTimePassed 0.0)
  (bind _returnvalue (Game|SpawnActorfromClass "/Game/blueprints/ShootingEnemy/BP_Shooting_Enemy_Projectile.BP_Shooting_Enemy_Projectile_C" (Transformation|GetActorTransform) "Undefined" "MultiplyWithRoot" 0 0))
  ;[1 1 1] Throws the Throwable at the player, with a specified air time (Time To Target)
  (bind _outlaunchvelocity (Class|GameplayStatics|SuggestProjectileVelocityMovingTarget (.location (Transformation|GetActorTransform)) (Game|GetPlayerCharacter 0) "0, 0, 0" 0.0 (Variables|Default|GetTimeToTarget) "None"))
  (bind _returnvalue_2 (AddComponent|AddProjectileMovementComponent _returnvalue))
  (Variables|/Script/Engine.MovementComponent|SetVelocity _returnvalue_2 _outlaunchvelocity))

(event Custom|Damage
  (params (damage :type Integer))
  (bind _output_get (Variables|Default|SetHealth (- (Variables|Default|GetHealth) damage)))
  (if (<= _output_get 0)
    (CallFunction|Die)
    (else
      (CallFunction|DamageEffect))))

(event Custom|DamageEffect)

(event Custom|DeathEffect)

(event EventTick
  (params (DeltaSeconds :type Float%20%28single-precision%29))
  (bind _returnvalue (Transformation|GetActorLocation))
  (bind _returnvalue_2 (Game|Player|GetPlayerPawn 0))
  (bind _returnvalue_3 (Transformation|GetActorLocation _returnvalue_2))
  (bind _returnvalue_4 (Math|Vector|Distance(Vector) _returnvalue_3 _returnvalue))
  (Variables|Default|SetTimePassed (+ (Variables|Default|GetTimePassed) DeltaSeconds))
  (Development|PrintString (Utilities|String|ToString(Float) _returnvalue_4))
  (if (<= _returnvalue_4 (Variables|Default|GetShootingRange))
    (Development|PrintString "face player")
    (CallFunction|FacePlayer)))

(fn ConstructionScript)

(fn FacePlayer
  (Transformation|SetActorRotation (Math|Conversions|RotationFromXVector (Math|Vector|RotateVector (Math|Vector|Normalize (* (- (Transformation|GetActorLocation (Game|Player|GetPlayerPawn 0)) (Transformation|GetActorLocation)) "1.000000,1.000000,0.000000")) "0, 0, 0"))))