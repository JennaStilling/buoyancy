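; Bowling ball enemy character that wanders to random nearby points until pawn sensing spots the player.
; It then chases via AI MoveTo and, within attack range, launches itself using a predicted velocity toward the moving target, destroying any player character its capsule hits.
; Launch state clears once it stops moving, and a failed chase drops aggro.
; The launch animation, damage and death hooks only add debug prints, with the latter two calling the parent.
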(event OnSeePawn(PawnSensing)
  (params (Pawn :type Pawn%20Object%20Reference))
  (Utilities|Casting|CastToBP_ThirdPersonCharacter Pawn)
  (Variables|Default|SetAggro true)
  (CallFunction|ChasePlayer))

(event OnComponentHit(CapsuleComponent)
  (params (HitComponent :type Primitive%20Component%20Object%20Reference) (OtherActor :type Actor%20Object%20Reference) (OtherComp :type Primitive%20Component%20Object%20Reference) (NormalImpulse :type Vector :default "0, 0, 0") (Hit :type Hit%20Result%20Structure%20%28by%20ref%29))
  (bind _asbp_third_person_character (Utilities|Casting|CastToBP_ThirdPersonCharacter OtherActor))
  (Actor|DestroyActor _asbp_third_person_character))

(event Custom|ChasePlayer
  (if (not (Variables|Default|GetLaunching))
    (if (Variables|Default|GetAggro)
      (AI|AIMoveTo self "0, 0, 0" (Game|Player|GetPlayerPawn 0) (Variables|Default|GetAttackRange) false
        (:OnSuccess
          (CallFunction|LaunchatPlayer))
        (:OnFail
          (Variables|Default|SetAggro false))))))

(event Custom|LaunchAtPlayer
  (Variables|Default|SetLaunched false)
  (Variables|Default|SetLaunching true)
  (CallFunction|PlayLaunchingAnimation)
  (Utilities|FlowControl|Delay (Variables|Default|GetAnimationDelay))
  (bind _outlaunchvelocity (Class|GameplayStatics|SuggestProjectileVelocityMovingTarget (.location (Transformation|GetActorTransform)) (Game|GetPlayerCharacter 0) "0, 0, 0" 0.0 (Variables|Default|GetTime%20to%20Target) "None"))
  (Character|LaunchCharacter _outlaunchvelocity false false)
  (Utilities|FlowControl|Delay (Variables|Default|GetAnimationDelay))
  (Utilities|FlowControl|Delay (Variables|Default|GetTime%20to%20Target))
  (Variables|Default|SetLaunched true))

(event Custom|PlayLaunchingAnimation
  (Utilities|FlowControl|Delay (Variables|Default|GetAnimationDelay))
  (Development|PrintString "Launch?"))

(event EventBeginPlay
  (|CallParentFunction) ; This node is disabled and will not be called.\nDrag off pins to build functionality.
)

(event Collision|EventActorBeginOverlap
  (params (OtherActor :type Actor%20Object%20Reference))
  (|CallParentFunction OtherActor) ; This node is disabled and will not be called.\nDrag off pins to build functionality.
)

(event EventTick
  (params (DeltaSeconds :type Float%20%28single-precision%29))
  (|CallParentFunction DeltaSeconds)
  (if (or (Variables|Default|GetLaunching) (Variables|Default|GetAggro))
    (if (Variables|Default|GetLaunched)
      (if (Math|Vector|VectorIsZero (Transformation|GetVelocity))
        (Variables|Default|SetLaunching false)))
    (else
      (Utilities|FlowControl|Delay 2.0)
      (AI|AIMoveTo self (.RandomLocation (AI|Navigation|GetRandomReachablePointinRadius (Transformation|GetActorLocation) 1e+03 0 0)) 0 5.0 false))))

(event EventDamageEffect
  (Development|PrintString (Utilities|String|Append "Bowling Health:" (Utilities|String|ToString(Integer) (Variables|Default|GetHealth))))
  (|CallParentFunction))

(event EventDeathEffect
  (Development|PrintString "Also Dead")
  (|CallParentFunction))

(fn ConstructionScript
  (|CallParentFunction))