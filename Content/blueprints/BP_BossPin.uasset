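; BP_BossPin is a destructible pin tied to the King Pin boss, damaged by player shots.
; Capsule overlaps with a player projectile or spray projectile each remove one point of the pin's Health.
; When Health runs out, it casts its Boss reference to BP_KingPin, takes one point from that boss's Health, prints the new value and destroys itself.
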(event OnComponentBeginOverlap(Capsule)
  (params (OverlappedComponent :type Primitive%20Component%20Object%20Reference) (OtherActor :type Actor%20Object%20Reference) (OtherComp :type Primitive%20Component%20Object%20Reference) (OtherBodyIndex :type Integer) (bFromSweep :type Boolean) (SweepResult :type Hit%20Result%20Structure%20%28by%20ref%29))
  (Utilities|Casting|CastToBP_PlayerProjectile OtherActor
    (:then
      _)
    (:CastFailed
      (Utilities|Casting|CastToBP_Spray_projectile OtherActor)))
  (bind _output_get (Variables|Default|SetHealth (- (Variables|Default|GetHealth) 1)))
  (if (<= _output_get 0)
    (bind _asbp_king_pin (Utilities|Casting|CastToBP_KingPin (Variables|Default|GetBoss)))
    (bind _output_get_2 (Variables|/Game/blueprints/BP_KingPin.BP_KingPin_C|SetHealth _asbp_king_pin (- (Variables|/Game/blueprints/BP_KingPin.BP_KingPin_C|GetHealth _asbp_king_pin) 1)))
    (Development|PrintString (Utilities|String|ToString(Integer) _output_get_2))
    (Actor|DestroyActor)))

(event EventBeginPlay)

(event Collision|EventActorBeginOverlap
  (params (OtherActor :type Actor%20Object%20Reference)))

(event EventTick
  (params (DeltaSeconds :type Float%20%28single-precision%29)))

(fn ConstructionScript)