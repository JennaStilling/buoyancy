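; BP_FloorPin is a short-lived actor that animates its ball, static meshes and spotlight vertically, then destroys itself.
; On BeginPlay it fires Kill and Light, each playing its own timeline.
; Kill drives the relative Z of Ball and four meshes from a scaled track and destroys the actor when finished.
; Light sets the spotlight's Z in world space, so that height ignores where the actor is placed.
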(event Custom|Kill
  (bind _ball (Variables|Default|Getball))
  (bind _staticmesh (Variables|Default|GetStaticMesh))
  (bind _staticmesh3 (Variables|Default|GetStaticMesh3))
  (bind _staticmesh2 (Variables|Default|GetStaticMesh2))
  (bind _staticmesh1 (Variables|Default|GetStaticMesh1))
  (bind _relativelocation (Variables|/Script/Engine.SceneComponent|GetRelativeLocation _staticmesh3))
  (bind _relativelocation_2 (Variables|/Script/Engine.SceneComponent|GetRelativeLocation _staticmesh1))
  (bind _relativelocation_3 (Variables|/Script/Engine.SceneComponent|GetRelativeLocation _ball))
  (bind _relativelocation_4 (Variables|/Script/Engine.SceneComponent|GetRelativeLocation _staticmesh2))
  (bind _relativelocation_5 (Variables|/Script/Engine.SceneComponent|GetRelativeLocation _staticmesh))
  (bind _newtrack_0 (Timeline|Timeline Play)
    (:Update
      (Transformation|SetRelativeLocation _ball (Math|Vector|MakeVector (.x _relativelocation_3) (.y _relativelocation_3) (* _newtrack_0 2.2e+02)) false false)
      (Transformation|SetRelativeLocation _staticmesh2 (Math|Vector|MakeVector (.x _relativelocation_4) (.y _relativelocation_4) (* _newtrack_0 2.2e+02)) false false)
      (Transformation|SetRelativeLocation _staticmesh (Math|Vector|MakeVector (.x _relativelocation_5) (.y _relativelocation_5) (* _newtrack_0 2.2e+02)) false false)
      (Transformation|SetRelativeLocation _staticmesh3 (Math|Vector|MakeVector (.x _relativelocation) (.y _relativelocation) (* _newtrack_0 2.2e+02)) false false)
      (Transformation|SetRelativeLocation _staticmesh1 (Math|Vector|MakeVector (.x _relativelocation_2) (.y _relativelocation_2) (* _newtrack_0 2.2e+02)) false false))
    (:Finished
      (Actor|DestroyActor))))

(event Custom|Light
  (bind _spotlight (Variables|Default|GetSpotLight))
  (bind _returnvalue (Transformation|GetWorldLocation _spotlight))
  (bind _newtrack_0 (Timeline|Timeline_0 Play)
    (:Update
      (Transformation|SetWorldLocation _spotlight (Math|Vector|MakeVector (.x _returnvalue) (.y _returnvalue) (* _newtrack_0 425.0)) false false))))

(event EventBeginPlay
  (CallFunction|Kill)
  (CallFunction|Light))

(event Collision|EventActorBeginOverlap
  (params (OtherActor :type Actor%20Object%20Reference)))

(event EventTick
  (params (DeltaSeconds :type Float%20%28single-precision%29)))

(fn ConstructionScript)