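; BP_gateway is a gate actor that opens and removes itself once its count of remaining enemies runs out.
; DecrementLeft lowers EnemiesLeft, which Tick polls every frame, calling AllDone whenever it is zero or below.
; AllDone plays a timeline that adds a scaled track value to the Cube's current relative Z on each update, so the offset accumulates, then destroys the actor when finished.
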(event Custom|AllDone
  (bind _cube (Variables|Default|GetCube))
  (bind _relativelocation (Variables|/Script/Engine.SceneComponent|GetRelativeLocation _cube))
  (bind _newtrack_0 (Timeline|Timeline Play)
    (:Update
      (Transformation|SetRelativeLocation _cube (Math|Vector|MakeVector (.x _relativelocation) (.y _relativelocation) (+ (.z _relativelocation) (* _newtrack_0 2e+02))) false false))
    (:Finished
      (Actor|DestroyActor))))

(event Custom|DecrementLeft
  (Variables|Default|SetenemiesLeft (- (Variables|Default|GetenemiesLeft) 1)))

(event EventBeginPlay)

(event Collision|EventActorBeginOverlap
  (params (OtherActor :type Actor%20Object%20Reference)))

(event EventTick
  (params (DeltaSeconds :type Float%20%28single-precision%29))
  (if (<= (Variables|Default|GetenemiesLeft) 0)
    (CallFunction|AllDone)))

(fn ConstructionScript)