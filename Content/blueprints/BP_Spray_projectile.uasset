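; Spray projectile that damages enemies derived from BPP_EnemyParent.
; A timeline, played from Tick, scales the projectile movement's max speed from InitialSpeed along a curve and destroys the actor when it finishes.
; Sphere overlaps ignore the third-person character and other spray projectiles; any other actor triggers a debug print and destroys the projectile, with enemies taking ProjectileDamage first.
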(event OnComponentBeginOverlap(Sphere)
  (params (OverlappedComponent :type Primitive%20Component%20Object%20Reference) (OtherActor :type Actor%20Object%20Reference) (OtherComp :type Primitive%20Component%20Object%20Reference) (OtherBodyIndex :type Integer) (bFromSweep :type Boolean) (SweepResult :type Hit%20Result%20Structure%20%28by%20ref%29))
  (Utilities|Casting|CastToBP_ThirdPersonCharacter OtherActor
    (:CastFailed
      (Utilities|Casting|CastToBP_Spray_projectile OtherActor
        (:CastFailed
          (Development|PrintString "Collided")
          (bind _asbpp_enemy_parent (Utilities|Casting|CastToBPP_EnemyParent OtherActor)
            (:then
              (Default|Damage _asbpp_enemy_parent (Variables|Default|GetProjectileDamage)))
            (:CastFailed
              _))
          (Actor|DestroyActor))))))

(event EventBeginPlay)

(event Collision|EventActorBeginOverlap
  (params (OtherActor :type Actor%20Object%20Reference)))

(event EventTick
  (params (DeltaSeconds :type Float%20%28single-precision%29))
  (bind _newtrack_0 (Timeline|Timeline Play)
    (:Update
      (Variables|/Script/Engine.ProjectileMovementComponent|SetMaxSpeed (Variables|Default|GetProjectileMovement) (* _newtrack_0 (Variables|Default|Getinitial%20speed))))
    (:Finished
      (Actor|DestroyActor))))

(fn ConstructionScript)