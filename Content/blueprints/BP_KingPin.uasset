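; KingPin boss that turns to face the player within arena range and attacks on a timer.
; A self-balancing random roll picks between up to three delayed floor pins, traced beneath the player, and two radial projectile volleys at player height; each pick lowers its own odds.
; At zero health, Tick triggers the cloth platform's death animation and a timeline Z move, then the kill plane's animation before destroying itself.
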(event Custom|Death%20animation
  (bind _defaultsceneroot (Variables|Default|GetDefaultSceneRoot))
  (bind _returnvalue (Transformation|GetWorldLocation _defaultsceneroot))
  (bind _newtrack_0 (Timeline|Timeline Play)
    (:Update
      (Transformation|SetWorldLocation _defaultsceneroot (Math|Vector|MakeVector (.x _returnvalue) (.y _returnvalue) (+ (* _newtrack_0 1e+02) (.z _returnvalue))) true false))
    (:Finished
      (bind _asbp_kill_plane (Utilities|Casting|CastToBP_killPlane (Variables|Default|GetKillPlane)))
      (Default|DeathAnim _asbp_kill_plane)
      (Actor|DestroyActor))))

(event Custom|ShootPins
  (bind _returnvalue (Transformation|GetActorTransform))
  (bind _returnvalue_2 (Transformation|GetActorTransform))
  (Variables|Default|SetAttackOdds (Math|Float|Clamp(Float) (+ (Variables|Default|GetAttackOdds) 0.1)))
  (Variables|Default|SettimePassed 0.0)
  (if (Utilities|IsValid (Game|Player|GetPlayerPawn 0))
    (for _index (range 0 36)
      (Game|SpawnActorfromClass "/Game/Blueprints/BP_BossProjectile.BP_BossProjectile_C" (Math|Transform|MakeTransform (Math|Vector|MakeVector (.x (.location _returnvalue)) (.y (.location _returnvalue)) (.z (Transformation|GetActorLocation (Game|Player|GetPlayerPawn 0)))) (Math|Rotator|MakeRotator 0.0 0.0 (+ (* _index 10) 0.0)) "1.000000,1.000000,1.000000") "Undefined" "MultiplyWithRoot" 0 0))
    (Utilities|FlowControl|Delay 2.5)
    (if (Utilities|IsValid (Game|Player|GetPlayerPawn 0))
      (for _index_2 (range 0 36)
        (Game|SpawnActorfromClass "/Game/Blueprints/BP_BossProjectile.BP_BossProjectile_C" (Math|Transform|MakeTransform (Math|Vector|MakeVector (.x (.location _returnvalue_2)) (.y (.location _returnvalue_2)) (.z (Transformation|GetActorLocation (Game|Player|GetPlayerPawn 0)))) (Math|Rotator|MakeRotator 0.0 0.0 (+ (* _index_2 10) 0.0)) "1.000000,1.000000,1.000000") "Undefined" "MultiplyWithRoot" 0 0)))))

(event Custom|FloorPins
  (bind _returnvalue (Game|Player|GetPlayerPawn 0))
  (bind _returnvalue_2 (Game|Player|GetPlayerPawn 0))
  (bind _returnvalue_3 (Game|Player|GetPlayerPawn 0))
  (bind _returnvalue_4 (Transformation|GetActorLocation _returnvalue))
  (bind _returnvalue_5 (Transformation|GetActorLocation _returnvalue_2))
  (bind _returnvalue_6 (Transformation|GetActorLocation _returnvalue_3))
  (Variables|Default|SetAttackOdds (Math|Float|Clamp(Float) (- (Variables|Default|GetAttackOdds) 0.1)))
  (Variables|Default|SettimePassed 0.0)
  (if (Utilities|IsValid (Game|Player|GetPlayerPawn 0))
    (bind (_outhit _returnvalue_7) (Collision|LineTraceByChannel (Math|Vector|MakeVector (.x _returnvalue_5) (.y _returnvalue_5) (.z _returnvalue_5)) (Math|Vector|MakeVector (.x _returnvalue_5) (.y _returnvalue_5) (- (.z _returnvalue_5) 1e+03)) "TraceTypeQuery1" false 0 "None"))
    (if _returnvalue_7
      (Game|SpawnActorfromClass "/Game/Blueprints/BP_FloorPin.BP_FloorPin_C" (Math|Transform|MakeTransform (.impactpoint _outhit)) "Undefined" "MultiplyWithRoot" 0 0)
      (Utilities|FlowControl|Delay 1.0)
      (bind (_outhit_2 _returnvalue_8) (Collision|LineTraceByChannel (Math|Vector|MakeVector (.x _returnvalue_6) (.y _returnvalue_6) (.z _returnvalue_6)) (Math|Vector|MakeVector (.x _returnvalue_6) (.y _returnvalue_6) (- (.z _returnvalue_6) 1e+03)) "TraceTypeQuery1" false 0 "None"))
      (if _returnvalue_8
        (Game|SpawnActorfromClass "/Game/Blueprints/BP_FloorPin.BP_FloorPin_C" (Math|Transform|MakeTransform (.impactpoint _outhit_2)) "Undefined" "MultiplyWithRoot" 0 0)
        (Utilities|FlowControl|Delay 1.0)
        (bind (_outhit_3 _returnvalue_9) (Collision|LineTraceByChannel (Math|Vector|MakeVector (.x _returnvalue_4) (.y _returnvalue_4) (.z _returnvalue_4)) (Math|Vector|MakeVector (.x _returnvalue_4) (.y _returnvalue_4) (- (.z _returnvalue_4) 1e+03)) "TraceTypeQuery1" false 0 "None"))
        (if _returnvalue_9
          (Game|SpawnActorfromClass "/Game/Blueprints/BP_FloorPin.BP_FloorPin_C" (Math|Transform|MakeTransform (.impactpoint _outhit_3)) "Undefined" "MultiplyWithRoot" 0 0))))))

(event EventBeginPlay)

(event Collision|EventActorBeginOverlap
  (params (OtherActor :type Actor%20Object%20Reference)))

(event EventTick
  (params (DeltaSeconds :type Float%20%28single-precision%29))
  (Variables|Default|SetTimePassed (+ (Variables|Default|GetTimePassed) DeltaSeconds))
  (if (Utilities|IsValid (Game|Player|GetPlayerPawn 0))
    (if (<= (Math|Vector|Distance(Vector) (Transformation|GetActorLocation (Game|Player|GetPlayerPawn 0)) (Transformation|GetActorLocation)) (Variables|Default|GetArenaRange))
      (CallFunction|FacePlayer)
      (if (<= (Variables|Default|GetAttackDelay) (Variables|Default|GettimePassed))
        (if (>= (Variables|Default|GetAttackOdds) (Math|Random|RandomFloat))
          (CallFunction|FloorPins)
          (else
            (CallFunction|ShootPins))))))
  (if (<= (Variables|Default|GetHealth) 0)
    (bind _asbp_cloth_platform (Utilities|Casting|CastToBP_clothPlatform (Variables|Default|Getcloth_platform)))
    (Default|DeathAnimation _asbp_cloth_platform)
    (CallFunction|DeathAnimation)))

(fn ConstructionScript)

(fn FacePlayer
  (Transformation|SetActorRotation (Math|Conversions|RotationFromXVector (Math|Vector|RotateVector (Math|Vector|Normalize (* (- (Transformation|GetActorLocation (Game|Player|GetPlayerPawn 0)) (Transformation|GetActorLocation)) "1.000000,1.000000,0.000000")) "0, 0, 0"))))