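; BP_BubblePool is a refill station that restores the third-person character's bubbles while the player stands in it.
; Sphere overlap events cast to BP_ThirdPersonCharacter, cache the player reference and toggle a flag on enter and exit.
; While flagged, Tick accumulates a timer and adds half a bubble each RefillTime interval until MaxBubbles is reached, printing debug messages along the way.
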(event OnComponentBeginOverlap(Sphere)
  (params (OverlappedComponent :type Primitive%20Component%20Object%20Reference) (OtherActor :type Actor%20Object%20Reference) (OtherComp :type Primitive%20Component%20Object%20Reference) (OtherBodyIndex :type Integer) (bFromSweep :type Boolean) (SweepResult :type Hit%20Result%20Structure%20%28by%20ref%29))
  (bind _asbp_third_person_character (Utilities|Casting|CastToBP_ThirdPersonCharacter OtherActor))
  (Variables|Default|SetPlayerRef _asbp_third_person_character)
  (Development|PrintString "Refilling bubbles")
  (Variables|Default|SetPlayerOnPool true))

(event OnComponentEndOverlap(Sphere)
  (params (OverlappedComponent :type Primitive%20Component%20Object%20Reference) (OtherActor :type Actor%20Object%20Reference) (OtherComp :type Primitive%20Component%20Object%20Reference) (OtherBodyIndex :type Integer))
  (Utilities|Casting|CastToBP_ThirdPersonCharacter OtherActor)
  (Development|PrintString "No longer refilling bubbles")
  (Variables|Default|SetPlayerOnPool false))

(event EventBeginPlay)

(event Collision|EventActorBeginOverlap
  (params (OtherActor :type Actor%20Object%20Reference)))

(event EventTick
  (params (DeltaSeconds :type Float%20%28single-precision%29))
  (bind _playerref (Variables|Default|GetPlayerRef))
  (if (Variables|Default|GetPlayerOnPool)
    (bind _output_get (Variables|Default|SetTimer (+ DeltaSeconds (Variables|Default|GetTimer))))
    (if (>= _output_get (Variables|Default|GetRefillTime))
      (Variables|Default|SetTimer 0.0)
      (if (>= (Variables|/Game/ThirdPerson/Blueprints/BP_ThirdPersonCharacter.BP_ThirdPersonCharacter_C|GetCurrentBubbles _playerref) (Variables|/Game/ThirdPerson/Blueprints/BP_ThirdPersonCharacter.BP_ThirdPersonCharacter_C|GetMaxBubbles _playerref))
        (Development|PrintString "Max bubbles")
        (else
          (bind _output_get_2 (Variables|/Game/ThirdPerson/Blueprints/BP_ThirdPersonCharacter.BP_ThirdPersonCharacter_C|SetCurrentBubbles _playerref (+ (Variables|/Game/ThirdPerson/Blueprints/BP_ThirdPersonCharacter.BP_ThirdPersonCharacter_C|GetCurrentBubbles _playerref) 0.5)))
          (Development|PrintString (Utilities|String|ToString(Float) _output_get_2)))))))

(fn ConstructionScript)